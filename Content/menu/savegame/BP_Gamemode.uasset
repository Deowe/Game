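; Game mode that saves and restores the player character's transform through a single save slot.
; On BeginPlay it loads the slot and applies the saved transform to the ThirdPersonCharacter's mesh component, not the actor, or creates the save file if none exists.
; The savegame event writes the current actor transform into the slot.
; Loadgame restarts the level to trigger that restore, while RestartLevel deletes the save before restarting.
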(event Custom|save%20game
  ;[1 1 1] save game
  (bind _returnvalue (SaveGame|LoadGamefromSlot "save1"))
  (bind _asbp_save_game (Utilities|Casting|CastTo _returnvalue))
  (Variables|Default|SetCharTransform _asbp_save_game (Transformation|GetActorTransform (.AsThird%20Person%20Character (Utilities|Casting|CastToThirdPersonCharacter (Game|GetPlayerCharacter 0)))))
  (SaveGame|SaveGametoSlot _asbp_save_game "save1"))

(event Custom|Load%20game
  ;[1 1 1] Load Game
  (Development|ExecuteConsoleCommand "RestartLevel" 0))

(event Custom|RestartLevel
  ;[1 1 1] delete save + restart
  (SaveGame|DeleteGameinSlot "save1")
  (Development|ExecuteConsoleCommand "RestartLevel" 0))

(event EventBeginPlay
  (bind _returnvalue (SaveGame|DoesSaveGameExist "save1"))
  (if _returnvalue
    ;[1 1 1] load game
    (bind _returnvalue_2 (SaveGame|LoadGamefromSlot "save1"))
    (bind _asbp_save_game (Utilities|Casting|CastTo _returnvalue_2))
    (bind _asthird_person_character (Utilities|Casting|CastToThirdPersonCharacter (Game|GetPlayerCharacter 0)))
    (Transformation|SetWorldTransform (Variables|/Script/Engine.Character|GetMesh _asthird_person_character) (Variables|Default|GetCharTransform _asbp_save_game) false false)
    (else
      ;[1 1 1] create save file
      (bind _returnvalue_3 (SaveGame|CreateSaveGameObject))
      (SaveGame|SaveGametoSlot _returnvalue_3 "save1"))))

(fn ConstructionScript)